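; BP_LoginPawn is a pawn that drives the front-end login and registration screens.
; On BeginPlay it creates the BP_Login widget, shows it and switches input to UI-only with an unlocked mouse.
; RegisterWidget hides login and creates a new BP_Registration widget on each call, while LoginWidget hides registration and reveals the stored login widget again.
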(event EventBeginPlay
  (bind _returnvalue (UserInterface|CreateWidget "/Game/Widget/BP_Login.BP_Login_C" (Game|GetPlayerController 0)))
  (bind _output_get (Variables|Default|SetLoginWidgetReg _returnvalue))
  (UserInterface|Viewport|AddtoViewport _output_get 0)
  (Input|SetInputModeUIOnly (Class|GameplayStatics|GetPlayerControllerfromID) 0 "DoNotLock"))

(event EventLoginWidget
  (Widget|SetVisibility (Variables|Default|GetLoginWidgetReg) "Visible")
  (Widget|SetVisibility (Variables|Default|GetRegistrationWidge) "Hidden"))

(event EventRegisterWidget
  (Widget|SetVisibility (Variables|Default|GetLoginWidgetReg) "Hidden")
  (bind _returnvalue (UserInterface|CreateWidget "/Game/Widget/BP_Registration.BP_Registration_C" (Game|GetPlayerController 0)))
  (bind _output_get (Variables|Default|SetRegistrationWidge _returnvalue))
  (UserInterface|Viewport|AddtoViewport _returnvalue 0))

(fn ConstructionScript)